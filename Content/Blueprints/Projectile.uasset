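; Projectile actor that detects overlaps with BP_Hatchback, though the successful cast currently triggers no further action.
; Tick runs through a 30-second Delay, then resets the actor's rotation to zero.
; Disconnected nodes would turn the projectile and hatchback meshes blue, and the hatchback red after a short delay, but they never run.
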(event Collision|EventActorBeginOverlap
  (params (OtherActor :type Actor%20Object%20Reference))
  (bind _asbp_hatchback (Utilities|Casting|CastToBP_Hatchback OtherActor)))

(event EventTick
  (params (DeltaSeconds :type Float%20%28single-precision%29))
  (Utilities|FlowControl|Delay 3e+01)
  (Transformation|SetActorRotation "0, 0, 0"))

(fn ConstructionScript
  (|CallParentFunction))