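; Red Dragon is a turret-style actor that faces the player's BP_Hatchback and plays a fire-breathing flight animation.
; BeginPlay caches the player pawn as the hatchback reference.
; Tick passes through a one-second Delay, then replays the animation once and snaps the static mesh's rotation from the spawn point toward the car.
; Bullet spawning with velocity-based target leading exists but is disconnected, so no projectiles are fired.
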(event EventTick
  (params (DeltaSeconds :type Float%20%28single-precision%29))
  ;[1 1 1] Turret Shooting
  (Utilities|FlowControl|Delay 1.0)
  (Components|Animation|PlayAnimation (Variables|Default|GetSkeletalMesh) "/Game/FourEvilDragonsHP/Animations/DragonTheUsurper/FlyFlameAnim.FlyFlameAnim" false)
  (Transformation|SetWorldRotation (Variables|Default|GetStaticMesh) (Math|Rotator|FindLookatRotation (Transformation|GetWorldLocation (Variables|Default|GetSpawnPoint)) (Transformation|GetWorldLocation (Variables|/Script/PhysXVehicles.WheeledVehicle|GetMesh (Variables|Default|GetPlayer%20Ref)))) false false))

(event EventBeginPlay
  ;[1 1 1] Turret Shooting
  (bind _asbp_hatchback (Utilities|Casting|CastToBP_Hatchback (Game|Player|GetPlayerPawn 0)))
  (Variables|Default|SetPlayer%20Ref _asbp_hatchback))

(fn ConstructionScript)