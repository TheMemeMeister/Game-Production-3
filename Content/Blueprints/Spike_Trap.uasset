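; Spike trap actor that damages the player's BP_Hatchback and swings a Knife mesh when its colliders are overlapped.
; TrapHitBox waits briefly, damages the car, sets HasTriggered and rotates the knife; later hits double the car's DmgPoints first.
; DoorCollider sets DmgPoints to 20 before triggering, while afterwards it delays, damages and rotates the knife.
; Each rotation is a single RInterpTo step, without Tick or Timeline.
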(event OnComponentBeginOverlap(TrapHitBox)
  (params (OverlappedComponent :type Primitive%20Component%20Object%20Reference) (OtherActor :type Actor%20Object%20Reference) (OtherComp :type Primitive%20Component%20Object%20Reference) (OtherBodyIndex :type Integer) (bFromSweep :type Boolean) (SweepResult :type Hit%20Result%20Structure%20%28by%20ref%29))
  (bind _knife (Variables|Default|GetKnife))
  (Utilities|FlowControl|Delay 1.0)
  ;[1 1 1] Rotating Knife and applying 10 dmg
  (if (Variables|Default|GetHasTriggered)
    ;[1 1 1] after rotation, have any additional collisions apply 20 dmg
    (bind _asbp_hatchback (Utilities|Casting|CastToBP_Hatchback (Game|Player|GetPlayerPawn 0)))
    (Variables|/Game/VehicleVarietyPack/Blueprints/Hatchback/BP_Hatchback.BP_Hatchback_C|SetDmgPoints _asbp_hatchback (* (Variables|/Game/VehicleVarietyPack/Blueprints/Hatchback/BP_Hatchback.BP_Hatchback_C|GetDmgPoints _asbp_hatchback) 2.0))
    (Default|ReduceHealth _asbp_hatchback (Variables|/Game/VehicleVarietyPack/Blueprints/Hatchback/BP_Hatchback.BP_Hatchback_C|GetHealth _asbp_hatchback))
    (Variables|Default|SetHasTriggered true)
    (Utilities|FlowControl|Delay 1.0)
    (else
      (bind _asbp_hatchback_2 (Utilities|Casting|CastToBP_Hatchback (Game|Player|GetPlayerPawn 0)))
      (Default|ReduceHealth _asbp_hatchback_2 (Variables|/Game/VehicleVarietyPack/Blueprints/Hatchback/BP_Hatchback.BP_Hatchback_C|GetHealth _asbp_hatchback_2))
      (Variables|Default|SetHasTriggered true)
      (Utilities|FlowControl|Delay 1.0)
      (Transformation|SetWorldRotation _knife (Math|Interpolation|RInterpTo (Transformation|GetWorldRotation _knife) "90.000000, 0,0.000000" (Utilities|Time|GetWorldDeltaSeconds) 1e+02) false false))))

(event OnComponentBeginOverlap(DoorCollider)
  (params (OverlappedComponent :type Primitive%20Component%20Object%20Reference) (OtherActor :type Actor%20Object%20Reference) (OtherComp :type Primitive%20Component%20Object%20Reference) (OtherBodyIndex :type Integer) (bFromSweep :type Boolean) (SweepResult :type Hit%20Result%20Structure%20%28by%20ref%29))
  (if (Variables|Default|GetHasTriggered)
    (Utilities|FlowControl|Delay 1.0)
    (bind _asbp_hatchback (Utilities|Casting|CastToBP_Hatchback (Game|Player|GetPlayerPawn 0)))
    (Default|ReduceHealth _asbp_hatchback (Variables|/Game/VehicleVarietyPack/Blueprints/Hatchback/BP_Hatchback.BP_Hatchback_C|GetHealth _asbp_hatchback))
    (Transformation|SetRelativeRotation (Variables|Default|GetKnife) (Math|Interpolation|RInterpTo (Transformation|GetWorldRotation (Variables|Default|GetKnife)) "0, 0, 0" (Utilities|Time|GetWorldDeltaSeconds) 1e+01) false false)
    (else
      (bind _asbp_hatchback_2 (Utilities|Casting|CastToBP_Hatchback (Game|Player|GetPlayerPawn 0)))
      (Variables|/Game/VehicleVarietyPack/Blueprints/Hatchback/BP_Hatchback.BP_Hatchback_C|SetDmgPoints _asbp_hatchback_2 2e+01)
      (Default|ReduceHealth _asbp_hatchback_2 (Variables|/Game/VehicleVarietyPack/Blueprints/Hatchback/BP_Hatchback.BP_Hatchback_C|GetHealth _asbp_hatchback_2)))))

(fn ConstructionScript)