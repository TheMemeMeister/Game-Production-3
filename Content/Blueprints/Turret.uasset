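; Turret actor that swivels its Body component to face the player's BP_Hatchback vehicle.
; Each Tick it casts the player pawn to BP_Hatchback and applies look-at pitch and yaw toward the car's mesh, preserving the Body's roll.
; The look-at starts from the Body's forward vector rather than its world location, so aim is computed from near the world origin.
; It contains no firing logic.
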(event EventBeginPlay)

(event Collision|EventActorBeginOverlap
  (params (OtherActor :type Actor%20Object%20Reference)))

(event EventTick
  (params (DeltaSeconds :type Float%20%28single-precision%29))
  (bind _body (Variables|Default|GetBody))
  (bind _asbp_hatchback (Utilities|Casting|CastToBP_Hatchback (Game|Player|GetPlayerPawn 0)))
  (Transformation|SetWorldRotation _body (Math|Rotator|MakeRotator (.roll (Transformation|GetWorldRotation _body)) (.pitch (Math|Rotator|FindLookatRotation (Math|Rotator|GetRotationXVector (Transformation|GetWorldRotation (Variables|Default|GetBody))) (Transformation|GetWorldLocation (Variables|/Script/PhysXVehicles.WheeledVehicle|GetMesh _asbp_hatchback)))) (.yaw (Math|Rotator|FindLookatRotation (Math|Rotator|GetRotationXVector (Transformation|GetWorldRotation (Variables|Default|GetBody))) (Transformation|GetWorldLocation (Variables|/Script/PhysXVehicles.WheeledVehicle|GetMesh _asbp_hatchback))))) false false))

(fn ConstructionScript)