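; Dragon enemy actor that attacks the player's BP_Hatchback with fireballs and dies when enough arrows hit it.
; Each tick it turns toward the car and line-traces to it; on a hit, a Delay throttles the attack animation and aimed Fireball spawn.
; Arrow overlaps reduce Health and update the AI_Health widget bar, with the actor destroyed and a death sound played at zero.
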(event EventTick
  (params (DeltaSeconds :type Float%20%28single-precision%29))
  (bind _spawnpoint (Variables|Default|GetSpawnPoint))
  (bind _returnvalue (Transformation|GetWorldLocation _spawnpoint))
  ;[0.2026 1 0.2461] Line Tracing for Dragons
  (CallFunction|SetDragonRotation)
  (bind _outhit (Collision|LineTraceByChannel (Transformation|GetWorldLocation (Variables|Default|GetSpawnPoint)) (Transformation|GetWorldLocation (Variables|/Script/PhysXVehicles.WheeledVehicle|GetMesh (Variables|Default|GetPlayer%20Ref))) "TraceTypeQuery1" false 0 "ForOneFrame"))
  (Utilities|Casting|CastToBP_Hatchback (.HitActor (Collision|BreakHitResult _outhit)))
  (Utilities|FlowControl|Delay 3.0)
  (Components|Animation|PlayAnimation (Variables|Default|GetSkeletalMesh) "/Game/FourEvilDragonsHP/Animations/DragonTheSoulEater/AttackFireBallAnim.AttackFireBallAnim" false)
  (Game|SpawnActorfromClass "/Game/Blueprints/Levels/TestServerItems/Fireball.Fireball_C" (Math|Transform|MakeTransform _returnvalue (Math|Rotator|FindLookatRotation _returnvalue (Transformation|GetWorldLocation (Variables|/Script/PhysXVehicles.WheeledVehicle|GetMesh (Variables|Default|GetPlayer%20Ref))))) "Undefined" 0 0))

(event Collision|EventActorBeginOverlap
  (params (OtherActor :type Actor%20Object%20Reference))
  ;[1 0.01618 0] Event Hit
  (Development|PrintString "You Hit Dragon")
  (Utilities|Casting|CastToArrow OtherActor)
  (CallFunction|ReduceHealth 1e+01)
  (bind _asai_health (Utilities|Casting|CastToAI_Health (UserInterface|GetUserWidgetObject (Variables|Default|GetHealth_Widget))))
  (Progress|SetPercent (Variables|/Game/Blueprints/UI/AI_Health.AI_Health_C|GetHealthBar _asai_health) (/ (Variables|Default|GetHealth) 1e+02)))

(event EventBeginPlay
  ;[0 0.4512 1] BeginPlay
  (Utilities|FlowControl|Sequence
    (:then_0
      (bind _asbp_hatchback (Utilities|Casting|CastToBP_Hatchback (Game|Player|GetPlayerPawn 0)))
      (Variables|Default|SetPlayer%20Ref _asbp_hatchback))
    (:then_1
      (bind _asai_health (Utilities|Casting|CastToAI_Health (UserInterface|GetUserWidgetObject (Variables|Default|GetHealth_Widget))))
      (Variables|/Game/Blueprints/UI/AI_Health.AI_Health_C|SetDragonRef _asai_health self))))

(fn ConstructionScript)

(fn ReduceHealth
  (params (Val :type Float%20%28single-precision%29))
  (bind _output_get (Variables|Default|SetHealth (- (Variables|Default|GetHealth) Val)))
  (if (<= _output_get 0.0)
    (Actor|DestroyActor)
    (Audio|PlaySound2D "/Game/Blueprints/Sound/dragondeath.dragondeath" 1.0 1.0 0.0 0 0)))

(fn SetDragonRotation
  (bind _staticmesh (Variables|Default|GetStaticMesh))
  (Transformation|SetWorldRotation _staticmesh (Math|Rotator|FindLookatRotation (Transformation|GetWorldLocation _staticmesh) (Transformation|GetWorldLocation (Variables|/Script/PhysXVehicles.WheeledVehicle|GetMesh (Variables|Default|GetPlayer%20Ref)))) false false))