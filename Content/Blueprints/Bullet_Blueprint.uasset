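; Bullet actor that damages the player's BP_Hatchback car when it overlaps a hatchback.
; On overlap it turns its own and the car's mesh red, restores the car to blue after a short delay, calls ReduceHealth on the player pawn rather than the overlapped car, then destroys itself.
; Tick resets rotation to zero behind a long Delay, and a hit-style custom event for destruction is kept for later use.
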(event Custom|CustomEvent
  (params (MyComp :type Primitive%20Component%20Object%20Reference) (Other :type Actor%20Object%20Reference) (OtherComp :type Primitive%20Component%20Object%20Reference) (bSelfMoved :type Boolean) (HitLocation :type Vector) (HitNormal :type Vector) (NormalImpulse :type Vector) (Hit :type Hit%20Result%20Structure%20%28by%20ref%29))
  ;[1 1 1] For later use to possibly destroy things
  (if (== Other OtherComp)
    (Actor|DestroyActor)
    (else
      (Utilities|FlowControl|Delay 1e+01)
      (Actor|DestroyActor))))

(event Collision|EventActorBeginOverlap
  (params (OtherActor :type Actor%20Object%20Reference))
  (bind _asbp_hatchback (Utilities|Casting|CastToBP_Hatchback OtherActor))
  (Rendering|Material|SetMaterial (Variables|Debug|GetStaticMeshComponent) 0 "/Game/FourEvilDragonsHP/Materials/DragonTheSoulEater/RedMat.RedMat")
  (Utilities|FlowControl|Delay 0.5)
  (Rendering|Material|SetMaterial (Variables|/Script/PhysXVehicles.WheeledVehicle|GetMesh _asbp_hatchback) 0 "/Game/FourEvilDragonsHP/Materials/DragonTheNightmare/BlueMat.BlueMat")
  (bind _asbp_hatchback_2 (Utilities|Casting|CastToBP_Hatchback (Game|Player|GetPlayerPawn 0)))
  (Default|ReduceHealth _asbp_hatchback_2 (Variables|/Game/VehicleVarietyPack/Blueprints/Hatchback/BP_Hatchback.BP_Hatchback_C|GetHealth _asbp_hatchback_2))
  (Actor|DestroyActor))

(event EventTick
  (params (DeltaSeconds :type Float%20%28single-precision%29))
  (Utilities|FlowControl|Delay 3e+01)
  (Transformation|SetActorRotation "0, 0, 0"))

(fn ConstructionScript)