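; Light switch Blueprint for the horror living room that flips its switch and turns its assigned lights on or off.
; SwitchLight passes through a short retriggerable delay into a FlipFlop that plays the SwitchMovement timeline forward or in reverse.
; The timeline rotates SwitchRoot on roll, and when it finishes in either direction it toggles the visibility of each valid entry in Lights.
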(event Custom|Switch%20Light
  ;[1 1 1] Rotate the Switch Component and toggle lightvisibility
  (Utilities|FlowControl|RetriggerableDelay 0.1)
  (Utilities|FlowControl|FlipFlop
    (:A
      (bind _switch_movement (Timeline|Switch%20Movement PlayFromStart)
        (:Update
          (Transformation|SetRelativeRotation (Variables|Default|GetSwitch_Root) (Math|Rotator|MakeRotator (Math|Float|Lerp 0.0 -47.0 _switch_movement) 0.0 0.0) false false))
        (:Finished
          (for _array_element (Variables|GeneralSettings|GetLights)
            (Utilities|IsValid _array_element
              (:Is%20Valid
                (Rendering|ToggleVisibility (Variables|/Script/Engine.Light|GetLightComponent _array_element) true)))))))
    (:B
      (Timeline|Switch%20Movement ReverseFromEnd))))

(fn ConstructionScript)