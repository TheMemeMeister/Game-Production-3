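; Modular radiator prop that assembles itself in the Construction Script from a configurable number of parts, with no runtime logic.
; A loop adds static mesh components spaced along local Y, picking each section randomly from four entries in a mesh array and capping the last with an end mesh.
; Optional feet are added at a set section interval, and disabling them destroys the existing feet component.
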(event EventBeginPlay)

(event Collision|EventActorBeginOverlap
  (params (OtherActor :type Actor%20Object%20Reference)))

(event EventTick
  (params (DeltaSeconds :type Float%20%28single-precision%29)))

(fn ConstructionScript
  (bind _add (LocalVariables|GetAdd))
  (bind _counter (LocalVariables|GetCounter))
  (bind _returnvalue (* _counter (.y (.location _add))))
  (bind _returnvalue_2 (Math|Transform|MakeTransform (Math|Vector|MakeVector (.x (.location _add)) _returnvalue (.z (.location _add))) (.rotation _add) (.scale _add)))
  (bind (_location _rotation _scale) (Math|Transform|BreakTransform _returnvalue_2))
  ;[1 1 1] Loops until Number of Radiator Parts is reached
  (while (!= (Variables|Generators|GetRadiator%20Parts) (LocalVariables|GetCounter))
    (Math|Integer|IncrementInt (LocalVariables|GetCounter)
      (:%20%20
        ;[1 1 1] If the last part is reached add end mesh
        (if (== (LocalVariables|GetCounter) (Variables|Generators|GetRadiator%20Parts))
          ;[1 1 1] Add end Mesh and Check if foot is enabled. If foot is disabled then destroy foot component
          (bind _returnvalue_3 (AddComponent|AddStaticMeshComponent false _returnvalue_2))
          (Components|StaticMesh|SetStaticMesh _returnvalue_3 (Variables|Internal|GetEnd))
          (if (not (Variables|Generators|GetEnable%20Feet))
            (Utilities|IsValid (Variables|Default|GetRadiator_feet_mesh)
              (:Is%20Valid
                (Components|DestroyComponent (Variables|Default|GetRadiator_feet_mesh)))))
          (else
            ;[1 1 1] Add Radiator Part at Position
            (bind _returnvalue_4 (AddComponent|AddStaticMeshComponent false _returnvalue_2))
            (Components|StaticMesh|SetStaticMesh _returnvalue_4 (Utilities|Array|Get(acopy) (Variables|Internal|GetRadiator_%20Array) (Math|Random|RandomInteger 4)))
            (if (Variables|Generators|GetEnable%20Feet)
              ;[1 1 1] Add Food Mesh at Position
              (bind _result (Math|Integer|IncrementInt (LocalVariables|GetCounter_Foot))
                (:%20%20
                  (if (and (Variables|Generators|GetEnable%20Feet) (== _result (Variables|Generators|GetFoot%20Amount)))
                    (bind _returnvalue_5 (AddComponent|AddStaticMeshComponent false (Math|Transform|MakeTransform (Math|Vector|MakeVector (.x _location) (+ (.y _location) -7.592319) (.z _location)) _rotation _scale)))
                    (Components|StaticMesh|SetStaticMesh _returnvalue_5 (Variables|Internal|GetFoot_mesh))
                    (LocalVariables|SetCounter_Foot 0))))
              (else
                (Utilities|FlowControl|DoOnce false
                  (:Completed
                    (Components|DestroyComponent (Variables|Default|GetRadiator_feet_mesh))))))))))))