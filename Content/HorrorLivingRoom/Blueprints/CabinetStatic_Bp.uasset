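; Configurable static cabinet prop for a living room scene, with four doors and two sliding boxes posed in the editor.
; The construction script optionally swaps the first two doors to glass meshes, then applies door yaws and box Y offsets, with the two box variables cross-assigned.
; Hide flags destroy child components of the matching door root or box, leaving that component itself.
; The event graph has no active logic.
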(event EventBeginPlay)

(event Collision|EventActorBeginOverlap
  (params (OtherActor :type Actor%20Object%20Reference)))

(event EventTick
  (params (DeltaSeconds :type Float%20%28single-precision%29)))

(fn ConstructionScript
  ;[1 1 1] Should Glassdoors be used ?
  (if (Variables|General|GetGlass%20Doors%20?)
    (Components|StaticMesh|SetStaticMesh (Variables|Default|Getcabinet_Door_1) "/Game/HorrorLivingRoom/Meshes/Cabinet/cabinet_glass_Door_1_mesh.cabinet_glass_Door_1_mesh")
    (Components|StaticMesh|SetStaticMesh (Variables|Default|Getcabinet_Door_2) "/Game/HorrorLivingRoom/Meshes/Cabinet/cabinet_glass_Door_2_mesh.cabinet_glass_Door_2_mesh"))
  ;[1 1 1] Set Door Rotation and Box Location if you want to open or close it
  (Transformation|SetRelativeLocation (Variables|Default|Getcabinet_Box_2) (Math|Vector|MakeVector 0.0 (Variables|Values|GetCabinet%20Box%201%20Location) 0.0) false false)
  (Transformation|SetRelativeLocation (Variables|Default|Getcabinet_Box_1) (Math|Vector|MakeVector 0.0 (Variables|Values|GetCabinet%20Box%202%20Location) 0.0) false false)
  (Transformation|SetRelativeRotation (Variables|Default|GetDoor1_Root) (Math|Rotator|MakeRotator 0.0 0.0 (Variables|Values|GetDoor%201%20Rotation)) false false)
  (Transformation|SetRelativeRotation (Variables|Default|GetDoor2_Root) (Math|Rotator|MakeRotator 0.0 0.0 (Variables|Values|GetDoor%202%20Rotation)) false false)
  (Transformation|SetRelativeRotation (Variables|Default|GetDoor3_Root) (Math|Rotator|MakeRotator 0.0 0.0 (Variables|Values|GetDoor%203%20Rotation)) false false)
  (Transformation|SetRelativeRotation (Variables|Default|GetDoor4_Root) (Math|Rotator|MakeRotator 0.0 0.0 (Variables|Values|GetDoor%204%20Rotation)) false false)
  ;[1 1 1] Hide Doors and Boxes you don't need
  (for (_array_element _array_index) (Utilities|Array|MakeArray (Variables|General|GetHide%20Door%201) (Variables|General|GetHide%20Door%202) (Variables|General|GetHide%20Door%203) (Variables|General|GetHide%20Door%204) (Variables|General|GetHide%20Box%201) (Variables|General|GetHide%20Box%202))
    (if _array_element
      (bind _output_get (LocalVariables|SetChild%20Components (Components|GetChildrenComponents (Utilities|Array|Get(acopy) (Utilities|Array|MakeArray (Variables|Default|GetDoor1_Root) (Variables|Default|GetDoor2_Root) (Variables|Default|GetDoor3_Root) (Variables|Default|GetDoor4_Root) (Variables|Default|GetCabinet%20Box%201) (Variables|Default|GetCabinet%20Box%202)) _array_index) true)))
      (for _array_element_2 _output_get
        (Components|DestroyComponent _array_element_2)))))