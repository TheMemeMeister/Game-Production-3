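; Procedural book prop that builds a randomized pile or shelf row of books in the Construction Script, with no active runtime logic.
; A loop adds static mesh components up to BooksCount, each with random scale, mesh and material, accumulating scaled book thickness along local Z for spacing.
; Pile mode randomizes XY offset and yaw, while shelf mode omits rotation and offsets each book by its scale, with random jitter only in X.
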(event EventBeginPlay)

(event Collision|EventActorBeginOverlap
  (params (OtherActor :type Actor%20Object%20Reference)))

(event EventTick
  (params (DeltaSeconds :type Float%20%28single-precision%29)))

(fn ConstructionScript
  ;[1 1 1] Loops until Books Count is reached
  (while (!= (Variables|General|GetBooks%20Count) (LocalVariables|GetCounter))
    ;[1 1 1] Should Books start as Pile or shelf ?
    (if (Variables|General|GetArrange%20as%20Pile%20?)
      ;[1 1 1] Set Random Values
      (LocalVariables|SetRandom%20Value (Math|Random|RandomFloatinRange (Variables|RandomBookValues|GetRandom%20Z%20Scale%20Min) (Variables|RandomBookValues|GetRandom%20Z%20Scale%20Max)))
      (LocalVariables|SetRandom%20Value%202 (Math|Random|RandomFloatinRange (Variables|RandomBookValues|GetRandom%20Y%20Scale%20Min) (Variables|RandomBookValues|GetRandom%20Y%20Scale%20Max)))
      ;[1 1 1] Add Current Distance multiplied with Random Value to the Book Size Array
      (Utilities|Array|Add (LocalVariables|GetSize_Array) (* 4.536259 (LocalVariables|GetRandom%20Value)))
      ;[1 1 1] Get the Current Booksize and add it to the Z Distance
      (Variables|Internal|SetBook%20Z%20Distance (+ (Utilities|Array|Get(acopy) (LocalVariables|GetSize_Array) (LocalVariables|GetCounter)) (Variables|Internal|GetBook%20Z%20Distance)))
      ;[1 1 1] Place Random Book At Position with Random Material and Increase Counter per one
      (bind _returnvalue (AddComponent|AddStaticMeshComponent false (Math|Transform|MakeTransform (Math|Vector|MakeVector (Math|Random|RandomFloatinRange (Variables|RandomBookValues|GetRandom%20Offset%20Min%20X) (Variables|RandomBookValues|GetRandom%20Offset%20Max%20X)) (Math|Random|RandomFloatinRange (Variables|IfPile|GetRandom%20Offset%20Min%20Y) (Variables|IfPile|GetRandom%20Offset%20Max%20Y)) (Variables|Internal|GetBook%20Z%20Distance)) (Math|Rotator|MakeRotator 0.0 0.0 (Math|Random|RandomFloatinRange (Variables|IfPile|GetRandom%20Rotation%20Min) (Variables|IfPile|GetRandom%20Rotation%20Max))) (Math|Vector|MakeVector (Math|Random|RandomFloatinRange (Variables|RandomBookValues|GetRandom%20X%20Scale%20Min) (Variables|RandomBookValues|GetRandom%20X%20Scale%20Max)) (LocalVariables|GetRandom%20Value%202) (LocalVariables|GetRandom%20Value)))))
      (Rendering|Material|SetMaterial _returnvalue 0 (Utilities|Array|Get(acopy) (LocalVariables|GetMaterials) (Math|Random|RandomInteger 3)))
      (Components|StaticMesh|SetStaticMesh _returnvalue (Utilities|Array|Get(acopy) (LocalVariables|GetBook_%20Array) (Math|Random|RandomInteger 7)))
      (Math|Integer|IncrementInt (LocalVariables|GetCounter))
      (else
        ;[1 1 1] Set Random Values
        (LocalVariables|SetRandom%20Value (Math|Random|RandomFloatinRange (Variables|RandomBookValues|GetRandom%20Z%20Scale%20Min) (Variables|RandomBookValues|GetRandom%20Z%20Scale%20Max)))
        (LocalVariables|SetRandom%20Value%202 (Math|Random|RandomFloatinRange (Variables|RandomBookValues|GetRandom%20Y%20Scale%20Min) (Variables|RandomBookValues|GetRandom%20Y%20Scale%20Max)))
        (LocalVariables|SetRandom%20Value%203 (Math|Random|RandomFloatinRange (Variables|RandomBookValues|GetRandom%20X%20Scale%20Min) (Variables|RandomBookValues|GetRandom%20X%20Scale%20Max)))
        ;[1 1 1] Add Current Distance multiplied with Random Value to the Book Size Array
        (Utilities|Array|Add (LocalVariables|GetSize_Array) (* 4.536259 (LocalVariables|GetRandom%20Value)))
        ;[1 1 1] Get the Current Booksize and add it to the Z Distance
        (Variables|Internal|SetBook%20Z%20Distance (+ (Utilities|Array|Get(acopy) (LocalVariables|GetSize_Array) (LocalVariables|GetCounter)) (Variables|Internal|GetBook%20Z%20Distance)))
        ;[1 1 1] Place Random Book At Position with Random Material and Increase Counter per one
        (bind _returnvalue_2 (AddComponent|AddStaticMeshComponent false (Math|Transform|MakeTransform (Math|Vector|MakeVector (+ (* 9.5 (LocalVariables|GetRandom%20Value%203)) (Math|Random|RandomFloatinRange (Variables|RandomBookValues|GetRandom%20Offset%20Min%20X) (Variables|RandomBookValues|GetRandom%20Offset%20Max%20X))) (* 14.0 (LocalVariables|GetRandom%20Value%202)) (Variables|Internal|GetBook%20Z%20Distance)) "0, 0, 0" (Math|Vector|MakeVector (LocalVariables|GetRandom%20Value%203) (LocalVariables|GetRandom%20Value%202) (LocalVariables|GetRandom%20Value)))))
        (Rendering|Material|SetMaterial _returnvalue_2 0 (Utilities|Array|Get(acopy) (LocalVariables|GetMaterials) (Math|Random|RandomInteger 3)))
        (Components|StaticMesh|SetStaticMesh _returnvalue_2 (Utilities|Array|Get(acopy) (LocalVariables|GetBook_%20Array) (Math|Random|RandomInteger 7)))
        (Math|Integer|IncrementInt (LocalVariables|GetCounter))))))