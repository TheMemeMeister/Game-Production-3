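; Configurable picture frame prop that displays a chosen image in one of several frame meshes.
; The Construction Script adds a static mesh component using the 1-based FrameNumber to pick from the Frames array.
; It creates a dynamic instance of material slot 1 and applies the image and normal textures.
; Per-frame arrays supply UV scale, offset and rotation to fit each mesh's UV layout; the event graph is empty.
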(event EventBeginPlay)

(event Collision|EventActorBeginOverlap
  (params (OtherActor :type Actor%20Object%20Reference)))

(event EventTick
  (params (DeltaSeconds :type Float%20%28single-precision%29)))

(fn ConstructionScript
  (bind _frames (Variables|Internal|GetFrames))
  (bind _frame_number (Variables|GeneralSettings|GetFrame%20Number))
  (bind _frame_number_2 (Variables|GeneralSettings|GetFrame%20Number))
  (bind _frame_number_3 (Variables|GeneralSettings|GetFrame%20Number))
  (bind _returnvalue (- _frame_number 1))
  (bind _returnvalue_2 (- _frame_number_2 1))
  (bind _returnvalue_3 (- _frame_number_3 1))
  (bind _output (Utilities|Array|Get(acopy) _frames _returnvalue_2))
  ;[1 1 1] Add Static Meshes and Change Dynamic Materials According to the Frames UV Map
  (bind _returnvalue_4 (AddComponent|AddStaticMeshComponent false))
  (bind _output_get (Variables|Default|SetFrame%20Mesh _returnvalue_4))
  (Components|StaticMesh|SetStaticMesh _output_get _output)
  (bind _returnvalue_5 (Rendering|Material|CreateDynamicMaterialInstance _output_get 1 (Rendering|Material|GetMaterial _output 1) "None" :!class /Script/Engine.PrimitiveComponent))
  (bind _output_get_2 (Variables|Internal|SetDynamic%20Material _returnvalue_5))
  (Rendering|Material|SetTextureParameterValue _output_get_2 "BaseColor" (Variables|GeneralSettings|GetImage%20Texture))
  (Rendering|Material|SetTextureParameterValue (Variables|Internal|GetDynamic%20Material) "Normal" (Variables|GeneralSettings|GetNormal%20Texture))
  (Rendering|Material|SetScalarParameterValue (Variables|Internal|GetDynamic%20Material) "UV Scale X" (Utilities|Array|Get(acopy) (Variables|Internal|GetUV%20Scale%20X) _returnvalue_3) :!class /Script/Engine.MaterialInstanceDynamic)
  (Rendering|Material|SetScalarParameterValue (Variables|Internal|GetDynamic%20Material) "UV Scale Y" (Utilities|Array|Get(acopy) (Variables|Internal|GetUV%20Scale%20Y) _returnvalue_3) :!class /Script/Engine.MaterialInstanceDynamic)
  (Rendering|Material|SetScalarParameterValue (Variables|Internal|GetDynamic%20Material) "V Offset" (Utilities|Array|Get(acopy) (Variables|Internal|GetV%20Offset) _returnvalue_3) :!class /Script/Engine.MaterialInstanceDynamic)
  (Rendering|Material|SetScalarParameterValue (Variables|Internal|GetDynamic%20Material) "U Offset" (Utilities|Array|Get(acopy) (Variables|Internal|GetU%20Offset) _returnvalue) :!class /Script/Engine.MaterialInstanceDynamic)
  (Rendering|Material|SetScalarParameterValue (Variables|Internal|GetDynamic%20Material) "UV Rotation" (Utilities|Array|Get(acopy) (Variables|Internal|GetUV%20Rotation) _returnvalue) :!class /Script/Engine.MaterialInstanceDynamic)
  (Rendering|Material|SetMaterial _output_get 1 (Variables|Internal|GetDynamic%20Material)))