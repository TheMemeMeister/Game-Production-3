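; Couch prop Blueprint for a horror living room set, with optional pillows that can be hidden per instance.
; The construction script loops over six HidePillow booleans and destroys the matching Pillow component for each one that is set.
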(fn ConstructionScript
  ;[1 1 1] Hide Pillows you don't need
  (for (_array_element _array_index) (Utilities|Array|MakeArray (Variables|General|GetHide%20Pillow%201) (Variables|General|GetHide%20Pillow%202) (Variables|General|GetHide%20Pillow%203) (Variables|General|GetHide%20Pillow%204) (Variables|General|GetHide%20Pillow%205) (Variables|General|GetHide%20Pillow%206))
    (if _array_element
      (Components|DestroyComponent (Utilities|Array|Get(acopy) (Utilities|Array|MakeArray (Variables|Default|GetPillow_1) (Variables|Default|GetPillow_2) (Variables|Default|GetPillow_3) (Variables|Default|GetPillow_4) (Variables|Default|GetPillow_5) (Variables|Default|GetPillow_6)) _array_index)))))