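; Rotary phone actor for the horror living room that animates its dial to dial a configurable number string.
; StartDial resets the dial, then replays the NumberDialTime timeline once per character, using each digit as an index into the Numbers array for the target yaw.
; The timeline's Dialing track drives the rotation lerp, and its Finished output advances the counter until the string ends.
; The construction script optionally removes the handset.
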(event Custom|Start%20Dial
  (bind _number_to_dial (Variables|General|GetNumber%20to%20dial))
  (bind _returnvalue (Utilities|String|GetCharacterArrayfromString _number_to_dial))
  ;[1 1 1] Check Number array and Rotate Dial
  (Transformation|SetRelativeRotation (Variables|Default|Getdial) "0, 0, 0" false false)
  (Variables|Internal|SetCounter 0)
  (bind _output_get (Variables|Internal|SetCounter%20max (Utilities|Array|Length _returnvalue)))
  (if (> _output_get 0)
    (bind _dialing (Timeline|Number%20Dial%20Time PlayFromStart)
      (:Update
        (Transformation|SetRelativeRotation (Variables|Default|Getdial) (Math|Rotator|MakeRotator 0.0 0.0 (Math|Float|Lerp 0.0 (Utilities|Array|Get(acopy) (Variables|Internal|GetNumbers) (Math|Conversions|ToInteger(Byte) (Utilities|Array|Get(acopy) _returnvalue (Variables|Internal|GetCounter)))) _dialing)) false false))
      (:Finished
        (bind _result (Math|Integer|IncrementInt (Variables|Internal|GetCounter))
          (:%20%20
            (if (not (== _result (Variables|Internal|GetCounter%20max)))
              (Timeline|Number%20Dial%20Time PlayFromStart))))))))

(event EventBeginPlay)

(event Collision|EventActorBeginOverlap
  (params (OtherActor :type Actor%20Object%20Reference)))

(event EventTick
  (params (DeltaSeconds :type Float%20%28single-precision%29)))

(fn ConstructionScript
  ;[1 1 1] Disable Handset
  (if (Variables|General|GetHide%20Handset)
    (Components|DestroyComponent (Variables|Default|Gethandset))))