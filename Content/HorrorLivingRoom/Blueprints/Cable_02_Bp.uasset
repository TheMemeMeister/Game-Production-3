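; Spline-driven cable actor for the Horror Living Room content that builds cable meshes along an editable path.
; The construction script fills the spline with spline mesh segments, sized manually or from the mesh bounds and multiplied by actor X scale.
; An optional Double flag adds a second mesh run with its own length settings.
; Each segment's start takes an adjustable offset, and tangents are clamped to segment length; there is no runtime logic.
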(event EventBeginPlay)

(event Collision|EventActorBeginOverlap
  (params (OtherActor :type Actor%20Object%20Reference)))

(event EventTick
  (params (DeltaSeconds :type Float%20%28single-precision%29)))

(fn ConstructionScript
  (if (Variables|General|GetDouble%20?)
    (Utilities|FlowControl|Sequence
      (:then_0
        (Variables|Secondary|SetSectionLength%202 (* (.x (Transformation|GetActorScale3D)) (Variables|Secondary|GetSectionLength%202)))
        (for _index (range 0 (Math|Float|Truncate (/ (Spline|GetSplineLength (Variables|Default|GetSpline)) (Variables|Secondary|GetSectionLength%202))))
          (bind _returnvalue (AddComponent|AddSplineMeshComponent false))
          (Components|StaticMesh|SetStaticMesh _returnvalue (Variables|Secondary|GetSecondary_Mesh%202))
          (SplineMesh|SetForwardAxis _returnvalue "X" true)
          (SplineMesh|SetStartandEnd _returnvalue (Spline|GetLocationatDistanceAlongSpline (Variables|Default|GetSpline) (+ (* _index (Variables|Secondary|GetSectionLength%202)) (Variables|Secondary|GetLenght%20Adjustment%202)) "Local") (Math|Vector|ClampVectorSize (Spline|GetTangentatDistanceAlongSpline (Variables|Default|GetSpline) (+ (* _index (Variables|Secondary|GetSectionLength%202)) (Variables|Secondary|GetLenght%20Adjustment%202)) "Local") 0.0 (- (Variables|Secondary|GetSectionLength%202) (Variables|Secondary|GetLenght%20Adjustment%202))) (Spline|GetLocationatDistanceAlongSpline (Variables|Default|GetSpline) (* (+ _index 1) (Variables|Secondary|GetSectionLength%202)) "Local") (Math|Vector|ClampVectorSize (Spline|GetTangentatDistanceAlongSpline (Variables|Default|GetSpline) (* (+ _index 1) (Variables|Secondary|GetSectionLength%202)) "Local") 0.0 (- (Variables|Secondary|GetSectionLength%202) (Variables|Secondary|GetLenght%20Adjustment%202))) true :!class /Script/Engine.SplineMeshComponent)))
      (:then_1
        (if (Variables|General|GetManual%20Segment%20Length%20?) :!label _label
          (Variables|General|SetSegment%20Length (Variables|General|GetSegment%20Length))
          (else
            (Variables|General|SetSegment%20Length (* (.x (.boxextent (StaticMesh|GetBounds (Variables|General|GetCable_Mesh)))) 2.0))))
        (Variables|General|SetSegment%20Length (* (.x (Transformation|GetActorScale3D)) (Variables|General|GetSegment%20Length)))
        (for _index_2 (range 0 (Math|Float|Truncate (/ (Spline|GetSplineLength (Variables|Default|GetSpline)) (Variables|General|GetSegment%20Length))))
          (bind _returnvalue_2 (AddComponent|AddSplineMeshComponent false))
          (Components|StaticMesh|SetStaticMesh _returnvalue_2 (Variables|General|GetCable_Mesh))
          (SplineMesh|SetForwardAxis _returnvalue_2 "X" true)
          (SplineMesh|SetStartandEnd _returnvalue_2 (Spline|GetLocationatDistanceAlongSpline (Variables|Default|GetSpline) (+ (* _index_2 (Variables|General|GetSegment%20Length)) (Variables|General|GetLenght%20Adjustment)) "Local") (Math|Vector|ClampVectorSize (Spline|GetTangentatDistanceAlongSpline (Variables|Default|GetSpline) (+ (* _index_2 (Variables|General|GetSegment%20Length)) (Variables|General|GetLenght%20Adjustment)) "Local") 0.0 (- (Variables|General|GetSegment%20Length) (Variables|General|GetLenght%20Adjustment))) (Spline|GetLocationatDistanceAlongSpline (Variables|Default|GetSpline) (* (+ _index_2 1) (Variables|General|GetSegment%20Length)) "Local") (Math|Vector|ClampVectorSize (Spline|GetTangentatDistanceAlongSpline (Variables|Default|GetSpline) (* (+ _index_2 1) (Variables|General|GetSegment%20Length)) "Local") 0.0 (- (Variables|General|GetSegment%20Length) (Variables|General|GetLenght%20Adjustment))) true :!class /Script/Engine.SplineMeshComponent))))
    (else
      (goto _label))))