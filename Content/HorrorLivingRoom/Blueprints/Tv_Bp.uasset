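; Television Blueprint for the horror living room that plays a movie on its screen when PlayMovieonTV is called.
; The event reveals red, green and blue spotlights and puts a dynamic material instance on the TV mesh's screen slot.
; It opens the video and a separate blur source on two media players, then starts both together after a short retriggerable delay.
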(event Custom|Play%20Movie%20on%20TV
  ;[1 1 1] Create Material Instances and Start Media Texture
  (Rendering|SetVisibility (Variables|Default|GetSpotLight_G) true true)
  (bind _returnvalue (Rendering|Material|CreateDynamicMaterialInstance (Variables|Default|GetTv_main_mesh) 1 (Rendering|Material|GetMaterial (Variables|Default|GetTv_main_mesh) 1) "None" :!class /Script/Engine.PrimitiveComponent))
  (Rendering|Material|SetMaterial (Variables|Default|GetTv_main_mesh) 1 _returnvalue)
  (Media|MediaPlayer|OpenSource (Variables|Media|GetMediaPlayer) (Variables|Media|GetVideo_Source))
  (Media|MediaPlayer|OpenSource (Variables|Media|GetMediaPlayer_Blur) (Variables|Media|GetBlur_Source))
  (Utilities|FlowControl|RetriggerableDelay 0.2)
  (Media|MediaPlayer|Play (Variables|Media|GetMediaPlayer) :!class /Script/MediaAssets.MediaPlayer)
  (Media|MediaPlayer|Play (Variables|Media|GetMediaPlayer_Blur) :!class /Script/MediaAssets.MediaPlayer))

(event Collision|EventActorBeginOverlap
  (params (OtherActor :type Actor%20Object%20Reference)))

(event EventTick
  (params (DeltaSeconds :type Float%20%28single-precision%29)))

(fn ConstructionScript)